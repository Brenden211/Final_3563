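; Interactable wooden door Blueprint that swings its mesh open and closed.
; An interact box overlap shows a widget and sets the in-range flag that gates the Open/Close event.
; That event toggles the closed state, plays a creak or close sound, and plays or reverses a timeline.
; The timeline lerps the mesh's relative rotation between the actor's rotation and a yaw offset from its initial rotation.
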(event OnComponentBeginOverlap(InteractBox)
  (params (OverlappedComponent :type Primitive%20Component%20Object%20Reference) (OtherActor :type Actor%20Object%20Reference) (OtherComp :type Primitive%20Component%20Object%20Reference) (OtherBodyIndex :type Integer) (bFromSweep :type Boolean) (SweepResult :type Hit%20Result%20Structure%20%28by%20ref%29))
  (Rendering|SetVisibility (Variables|Default|GetWidget) true true)
  (Variables|Default|SetInsideRadius true))

(event OnComponentEndOverlap(InteractBox)
  (params (OverlappedComponent :type Primitive%20Component%20Object%20Reference) (OtherActor :type Actor%20Object%20Reference) (OtherComp :type Primitive%20Component%20Object%20Reference) (OtherBodyIndex :type Integer))
  (Rendering|SetVisibility (Variables|Default|GetWidget) false true)
  (Variables|Default|SetInsideRadius false))

(event Custom|Open%20/%20Close
  (bind _returnvalue (Transformation|GetActorLocation))
  (bind _returnvalue_2 (Math|Rotator|MakeRotator 0.0 0.0 -2e+02))
  (bind _initialrotation (Variables|Default|GetInitialRotation))
  (bind _returnvalue_3 (Math|Rotator|CombineRotators _initialrotation _returnvalue_2))
  (if (Variables|Default|GetInsideRadius)
    (if (Variables|Default|GetIsClosed)
      (Variables|Default|SetTargetRoatation _returnvalue_3)
      (Variables|Default|SetIsClosed false)
      (Audio|PlaySoundatLocation "/Game/MyContent/Audio/SC_WoodenDoorOpenCreak.SC_WoodenDoorOpenCreak" _returnvalue "0, 0, 0" 1.0 1.0 0.0 0 0 0 0)
      (bind _dooranimation (Timeline|Timeline Play)
        (:Update
          (Transformation|SetRelativeRotation (Variables|Default|GetStaticMesh) (Math|Rotator|Lerp(Rotator) (Transformation|GetActorRotation) (Variables|Default|GetTargetRoatation) _dooranimation) false false)))
      (else
        (Variables|Default|SetTargetRoatation _returnvalue_3)
        (Variables|Default|SetIsClosed true)
        (Audio|PlaySoundatLocation "/Game/MyContent/Audio/SC_DoorClose.SC_DoorClose" _returnvalue "0, 0, 0" 1.0 1.0 0.0 0 0 0 0)
        (Timeline|Timeline Reverse)))))

(event EventBeginPlay
  (Utilities|FlowControl|Delay 0.2)
  (Variables|Default|SetInitialRotation (Transformation|GetActorRotation))
  (Rendering|SetVisibility (Variables|Default|GetWidget) false true))

(fn ConstructionScript)