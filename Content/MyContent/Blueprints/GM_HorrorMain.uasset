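; GM_HorrorMain is the horror game's main game mode, managing the objective HUD and the win screen.
; Four seconds after BeginPlay it creates the objective overlay widget, stores it as GameHUD and adds it to the viewport.
; The GameWon event shows the mouse cursor, switches input to UI only and displays the game-won widget.
; A separate ShowGameWon function only creates that widget and ends in an unused self-cast, leaving input unchanged.
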(event Custom|Event%20GameWon
  (bind _returnvalue (Game|GetPlayerController 0))
  (Variables|/Script/Engine.PlayerController|SetbShowMouseCursor _returnvalue true)
  (Input|SetInputModeUIOnly _returnvalue 0 "DoNotLock" false)
  (bind _returnvalue_2 (UserInterface|CreateWidget "/Game/MyContent/UI/WB_GameWon.WB_GameWon_C"))
  (UserInterface|Viewport|AddtoViewport _returnvalue_2 0))

(event EventBeginPlay
  (Utilities|FlowControl|Delay 4.0)
  (bind _returnvalue (UserInterface|CreateWidget "/Game/MyContent/UI/WB_ObjectiveOverlay.WB_ObjectiveOverlay_C"))
  (bind _output_get (Variables|Default|SetGameHUD _returnvalue))
  (UserInterface|Viewport|AddtoViewport _output_get 0))

(fn ConstructionScript)

(fn ShowGameWon
  (bind _returnvalue (UserInterface|CreateWidget "/Game/MyContent/UI/WB_GameWon.WB_GameWon_C"))
  (UserInterface|Viewport|AddtoViewport _returnvalue 0)
  (Utilities|Casting|CastToGM_HorrorMain (Game|GetGameMode)))