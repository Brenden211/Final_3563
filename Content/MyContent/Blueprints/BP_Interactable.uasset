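; BP_Interactable is a horror-game interactable actor that counts toward the win condition.
; Sphere overlaps show and hide its Widget, while IA_HorrorInteract calls OnInteract without checking overlap or prior interaction.
; OnInteract flags it used, increments GM_HorrorMain's InteractedCount, plays a click sound and updates the HUD text with the passed name.
; When that count equals InteractableCount, it calls the game mode's EventGameWon.
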(event OnComponentBeginOverlap(Sphere)
  (params (OverlappedComponent :type Primitive%20Component%20Object%20Reference) (OtherActor :type Actor%20Object%20Reference) (OtherComp :type Primitive%20Component%20Object%20Reference) (OtherBodyIndex :type Integer) (bFromSweep :type Boolean) (SweepResult :type Hit%20Result%20Structure%20%28by%20ref%29))
  (Rendering|SetVisibility (Variables|Components|GetWidget) true false))

(event OnComponentEndOverlap(Sphere)
  (params (OverlappedComponent :type Primitive%20Component%20Object%20Reference) (OtherActor :type Actor%20Object%20Reference) (OtherComp :type Primitive%20Component%20Object%20Reference) (OtherBodyIndex :type Integer))
  (Rendering|SetVisibility (Variables|Components|GetWidget) false false))

(event Input|EnhancedActionEvents|EnhancedInputActionIA_HorrorInteract
  (params (ActionValue :type Boolean) (ElapsedSeconds :type Float%20%28double-precision%29) (TriggeredSeconds :type Float%20%28double-precision%29) (InputAction :type Input%20Action%20Object%20Reference :default "/Game/MyContent/Input/Actions/IA_HorrorInteract.IA_HorrorInteract"))
  (CallFunction|OnInteract))

(fn ConstructionScript)

(fn OnInteract
  (params (OwnerName :type String))
  (Variables|Default|SetInteractableName OwnerName)
  (bind _asgm_horror_main (Utilities|Casting|CastToGM_HorrorMain (Game|GetGameMode)))
  (LocalVariables|SetGM_HorrorMainRef _asgm_horror_main)
  (Variables|Default|SetbHasBeenInteracted true)
  (bind _output_get (Variables|/Game/MyContent/Blueprints/GM_HorrorMain.GM_HorrorMain_C|SetInteractedCount (LocalVariables|GetGM_HorrorMainRef) (+ (Variables|/Game/MyContent/Blueprints/GM_HorrorMain.GM_HorrorMain_C|GetInteractedCount _asgm_horror_main) 1)))
  (Audio|PlaySoundatLocation "/Game/MyContent/Audio/Button_Click_Horror.Button_Click_Horror" (Transformation|GetActorLocation) "0, 0, 0" 1.0 1.0 0.0 0 0 0 0)
  (Utilities|Casting|CastToBP_HorrorPlayerFP (Game|GetPlayerCharacter 0))
  (Default|UpdateInteractText (Variables|/Game/MyContent/Blueprints/GM_HorrorMain.GM_HorrorMain_C|GetGameHUD (LocalVariables|GetGM_HorrorMainRef)) (Variables|Default|GetInteractableName))
  (if (== _output_get (Variables|/Game/MyContent/Blueprints/GM_HorrorMain.GM_HorrorMain_C|GetInteractableCount (LocalVariables|GetGM_HorrorMainRef)))
    (Default|EventGameWon (LocalVariables|GetGM_HorrorMainRef))))

(fn HasBeenInteracted
  (if (Variables|Default|GetbHasBeenInteracted)
    (return true)))