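; Pickup actor for a readable necklace note that shows a Necklace widget on screen.
; Box overlap shows and removes a WB_PickUpNote prompt, and the world Widget component is hidden at BeginPlay.
; The Notes event flip-flops between opening the widget with a paper sound while ignoring look and move input, and closing it.
; Separate PickUpNote and PutDownNote events only add or remove the widget; TogglePickUp does nothing.
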(event OnComponentBeginOverlap(Box)
  (params (OverlappedComponent :type Primitive%20Component%20Object%20Reference) (OtherActor :type Actor%20Object%20Reference) (OtherComp :type Primitive%20Component%20Object%20Reference) (OtherBodyIndex :type Integer) (bFromSweep :type Boolean) (SweepResult :type Hit%20Result%20Structure%20%28by%20ref%29))
  (bind _returnvalue (UserInterface|CreateWidget "/Game/MyContent/UI/WB_PickUpNote.WB_PickUpNote_C"))
  (UserInterface|Viewport|AddtoViewport _returnvalue 0))

(event OnComponentEndOverlap(Box)
  (params (OverlappedComponent :type Primitive%20Component%20Object%20Reference) (OtherActor :type Actor%20Object%20Reference) (OtherComp :type Primitive%20Component%20Object%20Reference) (OtherBodyIndex :type Integer))
  (Widget|RemovefromParent (stale OnComponentBeginOverlap(Box) _returnvalue)))

(event Custom|PickUpNote
  (bind _returnvalue (UserInterface|CreateWidget "/Game/NotePickUp/AllTheNotes/Necklace.Necklace_C"))
  (UserInterface|Viewport|AddtoViewport _returnvalue 0))

(event Custom|PutDownNote
  (Widget|RemovefromParent (stale Custom|PickUpNote _returnvalue)))

(event Custom|TogglePickUp
  (if (Variables|Default|GetisReading)
    _))

(event EventNotes
  (bind _returnvalue (Game|GetPlayerController 0))
  (Utilities|FlowControl|FlipFlop
    (:A
      (Audio|PlaySoundatLocation "/Game/NotePickUp/y2mate_com_-_Picking_up_paper_sound_effect.y2mate_com_-_Picking_up_paper_sound_effect" (Transformation|GetWorldLocation (Variables|Default|GetStaticMesh)) "0, 0, 0" 1.0 1.0 0.0 0 0 0 0)
      (bind _returnvalue_2 (UserInterface|CreateWidget "/Game/NotePickUp/AllTheNotes/Necklace.Necklace_C"))
      (UserInterface|Viewport|AddtoViewport _returnvalue_2 0)
      (Input|SetIgnoreLookInput _returnvalue true)
      (Input|SetIgnoreMoveInput _returnvalue true))
    (:B
      (Widget|RemovefromParent _returnvalue_2)
      (Input|SetIgnoreLookInput _returnvalue false)
      (Input|SetIgnoreMoveInput _returnvalue false))))

(event EventBeginPlay
  (Rendering|SetVisibility (Variables|Components|GetWidget) false false))

(fn ConstructionScript)